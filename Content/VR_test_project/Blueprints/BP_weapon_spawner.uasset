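; A VR weapon spawner actor with a world-space WBP_Gun_spawn menu that spawns the currently selected actor class.
; On BeginPlay it registers itself with the widget and starts a fast looping timer that yaws the menu toward the VR pawn's camera.
; Spawn_weapon line-traces along an arrow component and, on a hit, spawns the class slightly above the impact point.
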(event Custom|Trace_location_for_spawn
  (bind _arrow (Variables|Default|GetArrow))
  (bind _returnvalue (Transformation|GetWorldLocation _arrow))
  (bind (_outhit _returnvalue_2) (Collision|LineTraceByChannel _returnvalue (+ _returnvalue (* (Math|Vector|GetForwardVector (Transformation|GetWorldRotation _arrow)) 1.5e+03)) "TraceTypeQuery1" false 0 "None"))
  (if _returnvalue_2
    (bind _output_get (Variables|Default|SetLocation_to_spawn_current_weapon (Math|Vector|MakeVector (.X (Math|Vector|BreakVector (.ImpactPoint (Collision|BreakHitResult _outhit)))) (.Y (Math|Vector|BreakVector (.ImpactPoint (Collision|BreakHitResult _outhit)))) (+ (.Z (Math|Vector|BreakVector (.ImpactPoint (Collision|BreakHitResult _outhit)))) 45.0))))
    (Game|SpawnActorfromClass (Variables|Default|GetCurrent_actor_of_spawn) (Math|Transform|MakeTransform _output_get) "AlwaysSpawn" 0 0)))

(event Custom|Look_to_player
  (Transformation|SetWorldRotation (Variables|Default|GetWBP_gun_spawner) (Math|Rotator|MakeRotator 0.0 0.0 (.yaw (Math|Rotator|FindLookatRotation (Transformation|GetWorldLocation (Variables|Default|GetWBP_gun_spawner)) (Transformation|GetWorldLocation (Variables|/Game/VR_test_project/Blueprints/Pawns/VRPawn.VRPawn_C|GetCamera (Variables|Default|GetAs%20VRPawn)))))) false false))

(event Custom|Spawn_weapon
  (CallFunction|TraceLocationforSpawn))

(event EventBeginPlay
  (bind _asvrpawn (Utilities|Casting|CastToVRPawn (Game|Player|GetPlayerPawn 0)))
  (Variables|Default|SetAs%20VRPawn _asvrpawn)
  (bind _aswbp_gun_spawn (Utilities|Casting|CastToWBP_Gun_spawn (UserInterface|GetUserWidgetObject (Variables|Default|GetWBP_gun_spawner))))
  (Variables|/Game/VR_test_project/Blueprints/Widgets/WBP_Gun_spawn.WBP_Gun_spawn_C|SetCurrent_spawner _aswbp_gun_spawn self)
  (Utilities|Time|SetTimerbyFunctionName 0 "Look_to_player" 0.01 true))

(fn ConstructionScript)