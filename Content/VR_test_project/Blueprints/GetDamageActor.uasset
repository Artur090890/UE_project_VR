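; GetDamageActor is a damageable AI-movable pawn with a health component and a damage widget for a VR project.
; A polling timer waits for the player VRPawn's OverlapTriger flag, then stops and sends the pawn to a destination with AIMoveTo.
; A faster looping timer yaws the widget toward the player's camera.
; Taking any damage passes the health value to the widget.
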(event Custom|OverlapOrNot
  (if (Variables|/Game/VR_test_project/Blueprints/Pawns/VRPawn.VRPawn_C|GetOverlapTriger (Variables|Default|GetAs%20VRPawn))
    (Utilities|Time|ClearandInvalidateTimerbyHandle (Variables|Default|GetTimer))
    (AI|AIMoveTo self (Variables|Default|GetDestination) 0 5.0 false)))

(event Custom|Look_to_player
  (Transformation|SetWorldRotation (Variables|Default|GetWBP_damage) (Math|Rotator|MakeRotator 0.0 0.0 (.yaw (Math|Rotator|FindLookatRotation (Transformation|GetWorldLocation (Variables|Character|GetMesh)) (Transformation|GetWorldLocation (Variables|/Game/VR_test_project/Blueprints/Pawns/VRPawn.VRPawn_C|GetCamera (Variables|Default|GetAs%20VRPawn)))))) false false))

(event Game|Damage|EventAnyDamage
  (params (Damage :type Float%20%28single-precision%29) (DamageType :type Damage%20Type%20Object%20Reference) (InstigatedBy :type Controller%20Object%20Reference) (DamageCauser :type Actor%20Object%20Reference))
  (bind _aswbp_damage_character (Utilities|Casting|CastToWBP_damage_character (UserInterface|GetUserWidgetObject (Variables|Default|GetWBP_damage))))
  (Default|EventDamage _aswbp_damage_character (Variables|/Script/VR_test_project.YTHealthComponent|GetHealth (Variables|Default|GetYTHealth))))

(event EventBeginPlay
  (bind _asvrpawn (Utilities|Casting|CastToVRPawn (Game|Player|GetPlayerPawn 0)))
  (Variables|Default|SetAs%20VRPawn _asvrpawn)
  (bind _returnvalue (Utilities|Time|SetTimerbyFunctionName 0 "OverlapOrNot" 0.1 true))
  (Variables|Default|SetTimer _returnvalue)
  (Utilities|Time|SetTimerbyFunctionName 0 "Look_to_player" 0.01 true))

(fn ConstructionScript)