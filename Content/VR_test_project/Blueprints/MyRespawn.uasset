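; MyRespawn is a VR level-change actor that saves player state to the game instance before opening another level.
; BeginPlay links its WBP_change_level widget back to itself and, if FromAI is set, opens VRTemplateMap after a short delay.
; Execute_opening stores held weapon class and bullet count, checking the right hand only if the left is empty.
; It then records the pawn's location under the current level name and opens LevelName.
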(event Custom|Execute_opening
  (bind _as_bp_vrtest_instance (Variables|Default|GetAs%20BP%20VRTest%20Instance))
  (bind _as_bp_vrtest_instance_2 (Variables|Default|GetAs%20BP%20VRTest%20Instance))
  (bind _asvrpawn (Utilities|Casting|CastToVRPawn (Game|Player|GetPlayerPawn 0)))
  (Variables|Default|SetAs%20VRPawn _asvrpawn)
  (Utilities|FlowControl|Sequence
    (:then_0
      (Utilities|IsValid (Variables|/Game/VR_test_project/Blueprints/Pawns/VRPawn.VRPawn_C|GetHeldComponentLeft (Variables|Default|GetAs%20VRPawn))
        (:Is%20Valid
          (bind (_current_class _bullets) (Class|BPIWeaponData|GetWeaponData(Message) (Components|GetOwner (Variables|/Game/VR_test_project/Blueprints/Pawns/VRPawn.VRPawn_C|GetHeldComponentLeft (Variables|Default|GetAs%20VRPawn)))))
          (Variables|/Game/VR_test_project/Core/BP_VRTest_instance.BP_VRTest_instance_C|SetLeft_hand _as_bp_vrtest_instance_2 true)
          (Variables|/Game/VR_test_project/Core/BP_VRTest_instance.BP_VRTest_instance_C|SetBullet_count_left _as_bp_vrtest_instance_2 _bullets)
          (Variables|/Game/VR_test_project/Core/BP_VRTest_instance.BP_VRTest_instance_C|SetCurrent_weapon_class_left _as_bp_vrtest_instance_2 _current_class))
        (:Is%20Not%20Valid
          (Utilities|IsValid (Variables|/Game/VR_test_project/Blueprints/Pawns/VRPawn.VRPawn_C|GetHeldComponentRight (Variables|Default|GetAs%20VRPawn))
            (:Is%20Valid
              (bind (_current_class_2 _bullets_2) (Class|BPIWeaponData|GetWeaponData(Message) (Components|GetOwner (Variables|/Game/VR_test_project/Blueprints/Pawns/VRPawn.VRPawn_C|GetHeldComponentRight (Variables|Default|GetAs%20VRPawn)))))
              (Variables|/Game/VR_test_project/Core/BP_VRTest_instance.BP_VRTest_instance_C|SetRight_hand _as_bp_vrtest_instance true)
              (Variables|/Game/VR_test_project/Core/BP_VRTest_instance.BP_VRTest_instance_C|SetCurrent_weapon_class_right _as_bp_vrtest_instance _current_class_2)
              (Variables|/Game/VR_test_project/Core/BP_VRTest_instance.BP_VRTest_instance_C|SetBullet_count_right _as_bp_vrtest_instance _bullets_2))))))
    (:then_1
      (Utilities|FlowControl|Delay 0.1)
      (bind _returnvalue (Game|GetCurrentLevelName true))
      (Utilities|Map|Add (Variables|/Game/VR_test_project/Core/BP_VRTest_instance.BP_VRTest_instance_C|GetLevel_and_locations (Variables|Default|GetAs%20BP%20VRTest%20Instance)) (Utilities|String|StringToName _returnvalue) (Transformation|GetActorLocation (Variables|Default|GetAs%20VRPawn)))
      (Class|Respawn|OpenLevels (Variables|Default|GetLevel_name)))))

(event EventBeginPlay
  (bind _asbp_vrtest_instance (Utilities|Casting|CastToBP_VRTest_instance (Game|GetGameInstance)))
  (Variables|Default|SetAs%20BP%20VRTest%20Instance _asbp_vrtest_instance)
  (bind _aswbp_change_level (Utilities|Casting|CastToWBP_change_level (UserInterface|GetUserWidgetObject (Variables|Default|GetWidget))))
  (Variables|/Game/VR_test_project/Blueprints/Widgets/WBP_change_level.WBP_change_level_C|SetCurrent_menu _aswbp_change_level self)
  (Utilities|FlowControl|Delay 0.1)
  (if (Variables|Default|GetFrom_AI)
    (Class|Respawn|OpenLevels "VRTemplateMap")))

(event Collision|EventActorBeginOverlap
  (params (OtherActor :type Actor%20Object%20Reference)))

(event EventTick
  (params (DeltaSeconds :type Float%20%28single-precision%29)))

(fn ConstructionScript)